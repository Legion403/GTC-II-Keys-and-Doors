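; BP_CDPlayer is an interactable CD player that changes the game's music and tempo when used.
; BeginPlay applies its chosen material to Cube1 and caches the music handler, first-person character and fireshooter actors.
; Use passes its Music and BPM to the BPCSongSwitcher, starts a new clock at that BPM on the music handler, then calls SetClockPlayer on the character.
; PickUp returns a fixed enum value.
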(event `self.ReceiveBeginPlay`
  ; Set chosen Material
  (bind _output_get (set `self.Material` (`self.Material`)))
  (`PrimitiveComponent.SetMaterial` (`self.Cube1`) 0 _output_get)
  (bind _returnvalue (`GameplayStatics.GetActorOfClass` "/Game/Blueprints/Quartz/BP_MusicHandler.BP_MusicHandler_C"))
  (set `self.QuartzClockBPM` _returnvalue)
  (bind _returnvalue_2 (`GameplayStatics.GetActorOfClass` "/Game/FirstPerson/Blueprints/BP_FirstPersonCharacter.BP_FirstPersonCharacter_C"))
  (set `self.FirstPersonCharacter` _returnvalue_2)
  (bind _returnvalue_3 (`GameplayStatics.GetActorOfClass` "/Game/AI/BP_Fireshooter.BP_Fireshooter_C"))
  (set `self.Fireshooter` _returnvalue_3))

(event `/Game/Blueprints/BlueprintComponents/BPI_Interactable.Use`
  ;[0.04151 0.04894 0.15 0.5] Set BPM and plug into the BPC event
  (bind _output_get (set `self.BPM` (`self.BPM`)))
  (`/Game/MusicF/BPC_SongSwitcher.Change Song` (`self.BPC_SongSwitcher`) _output_get (`self.Music`))
  (`/Game/Blueprints/Quartz/BP_MusicHandler.StartNewClock` (`self.QuartzClockBPM`) _output_get)
  (`/Game/FirstPerson/Blueprints/BP_FirstPersonCharacter.Set Clock Player` (`self.FirstPersonCharacter`)))

(fn `PickUp`
  (returns (ItemType :type "/Game/Blueprints/E_Item Enum"))
  (return "NewEnumerator0"))

(fn `UserConstructionScript`)