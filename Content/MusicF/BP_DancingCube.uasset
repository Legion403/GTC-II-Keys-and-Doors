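; Cube actor that pulses and flashes to a music beat once ChangeBPM is called with a tempo.
; ChangeBPM and Timer call each other through a 60/BPM delay to form the beat loop.
; Each beat clears the material and restores the saved scale, then 0.1 seconds later applies Material_001_Inst and enlarges the cube.
; A timeline-driven bounce animation is present but never runs.
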(event `self.ChangeBPM`
  (params (BPM :type "Float (double-precision)"))
  (bind _cube (`self.Cube`))
  ;[0.0965 0.15 0.05289 0.5] Flash Color on Beat
  (`self.Timer`)
  (`PrimitiveComponent.SetMaterial` _cube 0 null)
  (`self.ScaleBToNormal`)
  (`KismetSystemLibrary.Delay` 0.1)
  (`PrimitiveComponent.SetMaterial` _cube 0 "/Game/TILESET/BoomboxHead/Materials/Material_001_Inst.Material_001_Inst")
  (`self.ScaleWBPM`))

(event `Timer`
  ;[0.0965 0.15 0.05289 0.5] Flash Color on Beat
  (`KismetSystemLibrary.Delay` (/ 60.0 (stale `self.ChangeBPM` BPM)))
  (`/Game/MusicF/BPI_BPMChanger.ChangeBPM` (stale `self.ChangeBPM` BPM)))

(event `self.ReceiveBeginPlay`
  (set `self.SavedInitalScale` (`SceneComponent.RelativeScale3D` (`self.Cube`))))

(event `ScaleWBPM`
  (bind _cube (`self.Cube`))
  (`SceneComponent.SetRelativeScale3D` _cube (* (`SceneComponent.RelativeScale3D` _cube) 1.1)))

(event `ScaleBToNormal`
  (`SceneComponent.SetRelativeScale3D` (`self.Cube`) (`self.SavedInitalScale`)))

(fn `UserConstructionScript`)