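; BP_WendigoShooterright is a ranged Wendigo enemy with events for throwing, cover search and random decisions.
; ThrowAttack plays a montage, then spawns an enemy fireball at its Box, toggling status flags.
; FlipACoin writes a random bool to the Blackboard, while FindCover records the nearest BP_Shelter.
; Only BP_PlayerDamage reduces health; a hit after reaching zero triggers a flame burst, soul spawn and destruction.
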(event `self.ReceiveBeginPlay`
  (set `self.Player` (`GameplayStatics.GetPlayerController` 0)))

(event `ThrowAttack`
  (set `self.ThrowFin` false)
  (set `self.Throwing` true)
  (`|PlayMontage` (`self.SkeletalMesh`) "/Game/3DObjects/Wendigostuff/Throwing_Montage.Throwing_Montage"
    (:`OnCompleted`
      (`|SpawnActorFromClass` "/Game/FirstPerson/Blueprints/HealthAndDamage/Projectiles/BP_FireballProjEnemy.BP_FireballProjEnemy_C" (`SceneComponent.K2_GetComponentToWorld` (`self.Box`)) "Undefined" "MultiplyWithRoot" null null)
      (set `self.Throwing` false)
      (set `self.ThrowFin` true))))

(event `FlipACoin`
  (bind _key_name (`self.Key Name`))
  (bind _returnvalue (`AIBlueprintHelperLibrary.GetBlackboard` (`AIBlueprintHelperLibrary.GetAIController` self)))
  (`KismetSystemLibrary.PrintString` "Flipping a coin!")
  (if (`KismetMathLibrary.RandomBool`)
    (bind _output_get (set `self.HeadsOrTails` true)) ; Heads
    (`BlackboardComponent.SetValueAsBool` _returnvalue _key_name _output_get)
    (else
      (bind _output_get_2 (set `self.HeadsOrTails` false)) ; Tails
      (`BlackboardComponent.SetValueAsBool` _returnvalue _key_name _output_get_2))))

(event `FindCover`
  (bind _outactors (`GameplayStatics.GetAllActorsOfClass` "/Game/Blueprints/BP_Shelter.BP_Shelter_C"))
  (for _array_element _outactors
    (bind _output_get (set `self.CurrentDistanceFromMe` (`self.GetDistanceTo` self _array_element)))
    (if (< _output_get (`self.ClosestDistance`))
      (set `self.ClosestDistance` (`self.CurrentDistanceFromMe`))
      (bind _output_get_2 (set `self.ClosestShelter` _array_element))
      (`KismetSystemLibrary.PrintString` (`KismetSystemLibrary.GetDisplayName` _output_get_2)))))

(event `self.ReceiveAnyDamage`
  (params (Damage :type "Float (single-precision)") (DamageType :type "DamageType Object Reference") (InstigatedBy :type "Controller Object Reference") (DamageCauser :type "Actor Object Reference"))
  (bind _returnvalue (`self.K2_GetActorLocation`))
  (if (== (`GameplayStatics.GetObjectClass` DamageType) "/Game/FirstPerson/Blueprints/HealthAndDamage/BP_PlayerDamage.BP_PlayerDamage_C")
    (if (`self.IsDead`)
      (`NiagaraFunctionLibrary.SpawnSystemAtLocation` "/Game/VFX/NS_FlameBurst.NS_FlameBurst" _returnvalue)
      (`KismetSystemLibrary.Delay` 0.2)
      (`|SpawnActorFromClass` "/Game/Blueprints/BP_Soul.BP_Soul_C" (`KismetMathLibrary.Conv_VectorToTransform` _returnvalue) "Undefined" "MultiplyWithRoot" null null)
      (`self.K2_DestroyActor`)
      (else
        (bind _output_get (set `self.CurrentHealth` (`KismetMathLibrary.FClamp` (- (`self.CurrentHealth`) Damage) 0.0 (`self.MaxHealth`))))
        (if (== _output_get 0.0)
          (set `self.IsDead` true))))))

(fn `UserConstructionScript`)