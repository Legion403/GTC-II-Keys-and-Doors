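; Fireshooter enemy that turns to face the first-person player, fires at them, and takes damage only from BP_PlayerDamage.
; A delayed Tick updates facing, eye effect positions and a lagged player location used as the beam's end.
; FireLaser, gated by a DoOnce, charges eye Niagara effects, then spawns a projectile and beam before cooling down.
; At zero health, the next player hit bursts it into flame and drops a BP_Lighter.
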(event `self.ReceiveBeginPlay`
  (bind _returnvalue (`GameplayStatics.GetActorOfClass` "/Game/FirstPerson/Blueprints/BP_FirstPersonCharacter.BP_FirstPersonCharacter_C"))
  (set `self.FirstPerson` _returnvalue))

(event `Fire Beam`
  (bind _returnvalue (`NiagaraFunctionLibrary.SpawnSystemAtLocation` "/Game/VFX/NS_Beam.NS_Beam" (`SceneComponent.K2_GetComponentLocation` (`self.Eye`))))
  (`NiagaraComponent.SetVariableVec3` _returnvalue "BeamEnd1" (`self.Delayed Player location`)))

(event `Link Eyes to body`
  (`SceneComponent.K2_SetWorldLocation` (`self.Niagara`) (`SceneComponent.K2_GetComponentLocation` (`self.Eye2`)) true false)
  (`SceneComponent.K2_SetWorldLocation` (`self.Niagara1`) (`SceneComponent.K2_GetComponentLocation` (`self.Eye3`)) true false))

(event `self.ReceiveTick`
  (params (DeltaSeconds :type "Float (single-precision)"))
  (`KismetSystemLibrary.Delay` 0.4)
  (`self.K2_SetActorRotation` (`KismetMathLibrary.FindLookAtRotation` (`self.K2_GetActorLocation`) (`self.K2_GetActorLocation` (`self.FirstPerson`))))
  (`self.Link Eyes to body`)
  (set `self.Delayed Player location` (`self.K2_GetActorLocation` (`self.FirstPerson`))))

(event `Fire Laser`
  (bind _eye1 (`self.Eye1`))
  (`/Engine/EditorBlueprintResources/StandardMacros.DoOnce` false :!label _label
    (:`Completed`
      (`ActorComponent.Activate` (`self.Niagara1`) false)
      (`ActorComponent.Activate` (`self.Niagara`) false)
      (`KismetSystemLibrary.Delay` 3.0)
      (`|SpawnActorFromClass` "/Game/Blueprints/BP_EnemyProjectile.BP_EnemyProjectile_C" (`KismetMathLibrary.MakeTransform` (`SceneComponent.K2_GetComponentLocation` _eye1) (`SceneComponent.K2_GetComponentRotation` _eye1)) "Undefined" "MultiplyWithRoot" null null)
      (`self.Fire Beam`)
      (`KismetSystemLibrary.Delay` 4.0)
      (goto _label :!via `Reset`))))

(event `self.ReceiveAnyDamage`
  (params (Damage :type "Float (single-precision)") (DamageType :type "DamageType Object Reference") (InstigatedBy :type "Controller Object Reference") (DamageCauser :type "Actor Object Reference"))
  (bind _returnvalue (`self.K2_GetActorLocation`))
  ; Death and Health
  (if (== (`GameplayStatics.GetObjectClass` DamageType) "/Game/FirstPerson/Blueprints/HealthAndDamage/BP_PlayerDamage.BP_PlayerDamage_C")
    (if (`self.IsDead`)
      (`NiagaraFunctionLibrary.SpawnSystemAtLocation` "/Game/VFX/NS_FlameBurst.NS_FlameBurst" _returnvalue)
      (`KismetSystemLibrary.Delay` 0.2)
      (`|SpawnActorFromClass` "/Game/Blueprints/BP_Lighter.BP_Lighter_C" (`KismetMathLibrary.Conv_VectorToTransform` _returnvalue) "Undefined" "MultiplyWithRoot" null null)
      (`self.K2_DestroyActor`)
      (else
        (bind _output_get (set `self.Current Health` (`KismetMathLibrary.FClamp` (- (`self.Current Health`) Damage) 0.0 (`self.Max Health`))))
        (if (== _output_get 0.0)
          (set `self.IsDead` true))))))

(fn `UserConstructionScript`)