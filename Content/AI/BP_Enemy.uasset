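; BP_Enemy is an enemy actor that takes damage from the player and leaves a soul behind when destroyed.
; Only BP_PlayerDamage lowers its clamped health; zero sets IsDead, and the next such hit spawns a flame burst, then BP_Soul after a short delay, and destroys it.
; BeginPlay deactivates BPDamager and caches the player controller, which Findtheplayeriflost uses as the target to turn toward.
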(event `self.ReceiveBeginPlay`
  (set `self.Player` (`GameplayStatics.GetPlayerController` 0))
  (`ActorComponent.Deactivate` (`self.BP_Damager`)))

(event `self.ReceiveAnyDamage`
  (params (Damage :type "Float (single-precision)") (DamageType :type "DamageType Object Reference") (InstigatedBy :type "Controller Object Reference") (DamageCauser :type "Actor Object Reference"))
  (bind _returnvalue (`self.K2_GetActorLocation`))
  (if (== (`GameplayStatics.GetObjectClass` DamageType) "/Game/FirstPerson/Blueprints/HealthAndDamage/BP_PlayerDamage.BP_PlayerDamage_C")
    (if (`self.IsDead`)
      (`NiagaraFunctionLibrary.SpawnSystemAtLocation` "/Game/VFX/NS_FlameBurst.NS_FlameBurst" _returnvalue)
      (`KismetSystemLibrary.Delay` 0.2)
      (`|SpawnActorFromClass` "/Game/Blueprints/BP_Soul.BP_Soul_C" (`KismetMathLibrary.Conv_VectorToTransform` _returnvalue) "Undefined" "MultiplyWithRoot" null null)
      (`self.K2_DestroyActor`)
      (else
        (bind _output_get (set `self.Current Health` (`KismetMathLibrary.FClamp` (- (`self.Current Health`) Damage) 0.0 (`self.Max Health`))))
        (if (== _output_get 0.0)
          (set `self.IsDead` true))))))

(event `Find the player if lost`
  (`self.K2_SetActorRotation` (`KismetMathLibrary.FindLookAtRotation` (`self.K2_GetActorLocation`) (`self.K2_GetActorLocation` (`self.Player`)))))

(fn `UserConstructionScript`)