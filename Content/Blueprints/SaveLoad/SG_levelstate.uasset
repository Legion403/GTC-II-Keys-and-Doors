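; SG_levelstate is a save/load Blueprint that records level state as lists of activated actors and inventories.
; AddActor and AddInventory append unique entries, and ActivateActors replays the saved state by calling ActivateMessage on each stored actor.
; LoadInventories is unfinished: it loops over the separate InvActors map with no loop body, leaving enum-inventory lookups unconnected.
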(event `AddActor`
  (params (NewItem :type "Actor Object Reference (by ref)"))
  (`KismetArrayLibrary.Array_AddUnique` (`self.ActivatedActors`) NewItem))

(event `ActivateActors`
  (for _array_element (`self.ActivatedActors`)
    (message `/Game/Blueprints/SaveLoad/BPI_Activated.Activate` _array_element)))

(event `Add Inventory`
  (params (Inventory :type "/Game/Blueprints/BPC_Inventory Object Reference (by ref)"))
  (`KismetArrayLibrary.Array_AddUnique` (`self.Inventories`) Inventory))

(event `Load Inventories`
  (bind (_keypin _valuepin) (`|MapForEach` (`self.InvActors`))))