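; Door actor that plays an opening animation and sound, then disables its box collision to clear the way.
; OpenDoor does this once, only if the cached first-person character has a key, and consumes it.
; JustOpen opens without a key check and adds the door to GM_SaveLoad's LevelState.
; Activate calls both in sequence, so it opens the door even without a key.
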(event `self.ReceiveBeginPlay`
  (bind _asbp_first_person_character (cast `/Game/FirstPerson/Blueprints/BP_FirstPersonCharacter` (`GameplayStatics.GetPlayerCharacter` 0)))
  (set `self.As BP First Person Character` _asbp_first_person_character))

(event `Open Door`
  (bind _as_bp_first_person_character (`self.As BP First Person Character`))
  (if (`/Game/FirstPerson/Blueprints/BP_FirstPersonCharacter.HasKey` _as_bp_first_person_character)
    (`/Engine/EditorBlueprintResources/StandardMacros.DoOnce` false
      (:`Completed`
        (`SkeletalMeshComponent.PlayAnimation` (`self.Door`) "/Game/3DObjects/Door/SkeletalMeshes/Door_Anim.Door_Anim" false)
        (`GameplayStatics.PlaySound2D` "/Game/SoundEffects/131029__dymewiz__locking-a-door_02.131029__dymewiz__locking-a-door_02" 1.0 1.0 0.0 null null)
        (`PrimitiveComponent.SetCollisionEnabled` (`self.Box`) "NoCollision")
        (set `/Game/FirstPerson/Blueprints/BP_FirstPersonCharacter.HasKey` false _as_bp_first_person_character)))))

(event `/Game/Blueprints/SaveLoad/BPI_Activated.Activate`
  (`self.Open Door`)
  (`self.JustOpen`))

(event `JustOpen`
  (`SkeletalMeshComponent.PlayAnimation` (`self.Door`) "/Game/3DObjects/Door/SkeletalMeshes/Door_Anim.Door_Anim" false)
  (`GameplayStatics.PlaySound2D` "/Game/SoundEffects/131029__dymewiz__locking-a-door_02.131029__dymewiz__locking-a-door_02" 1.0 1.0 0.0 null null)
  (`PrimitiveComponent.SetCollisionEnabled` (`self.Box`) "NoCollision")
  (bind _asgm_save_load (cast `/Game/Blueprints/GM_SaveLoad` (`GameplayStatics.GetGameMode`)))
  (`/Game/Blueprints/SaveLoad/SG_levelstate.AddActor` (`/Game/Blueprints/GM_SaveLoad.LevelState` _asgm_save_load) self)
  (`KismetSystemLibrary.Delay` 0.2))

(fn `UserConstructionScript`)