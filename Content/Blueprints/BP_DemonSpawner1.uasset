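; BP_DemonSpawner1 is an encounter trigger that summons demons once and later drops a key.
; The player's first overlap with E runs SummonDemons, spawning enemies at tagged components plus fireshooters, shelters and Wendigo shooters at their spawner actors, with flame bursts.
; A delayed Tick polls whether any BP_Enemy remains.
; Overlapping again after none remain spawns BP_Key and destroys the spawner.
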(event `Summon Demons`
  (for _array_element (`self.GetComponentsByTag` "/Script/Engine.ActorComponent" "Spawnpoint")
    (bind _asscene_component (cast `SceneComponent` _array_element))
    (bind _returnvalue (`SceneComponent.K2_GetComponentLocation` _asscene_component))
    (bind _returnvalue_2 (`|SpawnActorFromClass` "/Game/AI/BP_Enemy.BP_Enemy_C" (`KismetMathLibrary.Conv_VectorToTransform` _returnvalue) "Undefined" "MultiplyWithRoot" null null))
    (`NiagaraFunctionLibrary.SpawnSystemAtLocation` "/Game/VFX/NS_FlameBurst.NS_FlameBurst" _returnvalue))
  (`ActorComponent.Activate` (`/Game/AI/BP_Enemy.BP_Damager` _returnvalue_2) false)
  (bind _outactors (`GameplayStatics.GetAllActorsOfClass` "/Game/Blueprints/BP_GargoyleSpawner.BP_GargoyleSpawner_C"))
  (for _array_element_2 _outactors
    (bind _returnvalue_3 (`SceneComponent.K2_GetComponentLocation` (`/Game/Blueprints/BP_GargoyleSpawner.SpawnPoint` _array_element_2)))
    (`|SpawnActorFromClass` "/Game/AI/BP_Fireshooter.BP_Fireshooter_C" (`KismetMathLibrary.Conv_VectorToTransform` _returnvalue_3) "Undefined" "MultiplyWithRoot" null null)
    (`NiagaraFunctionLibrary.SpawnSystemAtLocation` "/Game/VFX/NS_FlameBurst.NS_FlameBurst" _returnvalue_3))
  (bind _outactors_2 (`GameplayStatics.GetAllActorsOfClass` "/Game/Blueprints/BP_ShelterSpawner.BP_ShelterSpawner_C"))
  (for _array_element_3 _outactors_2
    (bind _returnvalue_4 (`SceneComponent.K2_GetComponentLocation` (`/Game/Blueprints/BP_ShelterSpawner.Spawne Point` _array_element_3)))
    (`|SpawnActorFromClass` "/Game/Blueprints/BP_Shelter.BP_Shelter_C" (`KismetMathLibrary.Conv_VectorToTransform` _returnvalue_4) "Undefined" "MultiplyWithRoot" null null)
    (`NiagaraFunctionLibrary.SpawnSystemAtLocation` "/Game/VFX/NS_FlameBurst.NS_FlameBurst" _returnvalue_4))
  (bind _outactors_3 (`GameplayStatics.GetAllActorsOfClass` "/Game/Blueprints/BP_WendigoSpawner.BP_WendigoSpawner_C"))
  (for _array_element_4 _outactors_3
    (bind _returnvalue_5 (`SceneComponent.K2_GetComponentLocation` (`/Game/Blueprints/BP_WendigoSpawner.SpawnPoint` _array_element_4)))
    (`|SpawnActorFromClass` "/Game/AI/BP_WendigoShooterright.BP_WendigoShooterright_C" (`KismetMathLibrary.Conv_VectorToTransform` _returnvalue_5) "Undefined" "MultiplyWithRoot" null null)
    (`NiagaraFunctionLibrary.SpawnSystemAtLocation` "/Game/VFX/NS_FlameBurst.NS_FlameBurst" _returnvalue_5))
  (set `self.SpawnedEnemies` true))

(event `self.e.OnComponentBeginOverlap`
  (params (OverlappedComponent :type "PrimitiveComponent Object Reference") (OtherActor :type "Actor Object Reference") (OtherComp :type "PrimitiveComponent Object Reference") (OtherBodyIndex :type Integer) (bFromSweep :type Boolean) (SweepResult :type "HitResult Structure (by ref)"))
  (if (and (`self.NoEnemiesLeft`) (`self.SpawnedEnemies`))
    (`|SpawnActorFromClass` "/Game/Blueprints/BP_Key.BP_Key_C" (`SceneComponent.K2_GetComponentToWorld` (`self.Key Spawn`)) "Undefined" "MultiplyWithRoot" null null)
    (`KismetSystemLibrary.Delay` 0.2)
    (`self.K2_DestroyActor`)
    (else
      (`/Engine/EditorBlueprintResources/StandardMacros.DoOnce` false
        (:`Completed`
          (cast `/Game/FirstPerson/Blueprints/BP_FirstPersonCharacter` OtherActor)
          (`ActorComponent.Activate` (`self.Niagara`) false)
          (`KismetSystemLibrary.Delay` 1.0)
          (`self.Summon Demons`))))))

(event `self.ReceiveTick`
  (params (DeltaSeconds :type "Float (single-precision)"))
  (`KismetSystemLibrary.Delay` 1.0)
  (bind _outactors (`GameplayStatics.GetAllActorsOfClass` "/Game/AI/BP_Enemy.BP_Enemy_C"))
  (set `self.NoEnemiesLeft` (`KismetArrayLibrary.Array_IsEmpty` _outactors)))

(fn `UserConstructionScript`)