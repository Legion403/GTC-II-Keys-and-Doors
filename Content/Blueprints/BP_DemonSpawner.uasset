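; BP_DemonSpawner is a one-shot trigger that spawns an enemy when the player walks into it.
; An overlap on component E passes a DoOnce before the cast to BP_FirstPersonCharacter, so any first overlapping actor uses up the trigger.
; For the player, it activates its Niagara effect, waits briefly, then SummonDemons spawns one BP_Enemy and a flame burst at SpawnPoint.
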(event `Summon Demons`
  (bind _returnvalue (`SceneComponent.K2_GetComponentLocation` (`self.Spawn Point`)))
  (`|SpawnActorFromClass` "/Game/AI/BP_Enemy.BP_Enemy_C" (`KismetMathLibrary.Conv_VectorToTransform` _returnvalue) "Undefined" "MultiplyWithRoot" null null)
  (`NiagaraFunctionLibrary.SpawnSystemAtLocation` "/Game/VFX/NS_FlameBurst.NS_FlameBurst" _returnvalue))

(event `self.e.OnComponentBeginOverlap`
  (params (OverlappedComponent :type "PrimitiveComponent Object Reference") (OtherActor :type "Actor Object Reference") (OtherComp :type "PrimitiveComponent Object Reference") (OtherBodyIndex :type Integer) (bFromSweep :type Boolean) (SweepResult :type "HitResult Structure (by ref)"))
  (`/Engine/EditorBlueprintResources/StandardMacros.DoOnce` false
    (:`Completed`
      (cast `/Game/FirstPerson/Blueprints/BP_FirstPersonCharacter` OtherActor)
      (`ActorComponent.Activate` (`self.Niagara`) false)
      (`KismetSystemLibrary.Delay` 1.0)
      (`self.Summon Demons`))))

(fn `UserConstructionScript`)