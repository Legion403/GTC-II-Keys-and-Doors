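; Stats component that holds a character's health, mana, stamina, experience, gold and saved location in a single Stats struct.
; GetCanSPrint reports whether stamina is above one, and Sprinting subtracts a given drain from stamina while keeping the other fields.
; Every tick, a debug event prints the stats other than saved location as on-screen text lasting one frame's delta time.
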(event `self.ReceiveTick`
  (params (DeltaSeconds :type "Float (single-precision)"))
  (`self.Debug Stats` DeltaSeconds))

(event `Debug Stats`
  (params (Duration :type "Float (double-precision)"))
  (bind (_health _mana _savedlocation _gold _experience _stamina) (break `/Game/Blueprints/BlueprintComponents/S_Stats` (`self.Stats`)))
  (`KismetSystemLibrary.PrintText` (`|FormatText` "HP {Health}, MP: {Mana}, SP: {Stamina}XP: {Experience}, Gold: {Gold}" _health _mana _experience _gold _stamina) true true (struct :`R` 1.0 :`G` 0.058461 :`A` 1.0) Duration))

(fn `GetCanSPrint`
  (returns (CanSprint :type Boolean))
  (return (> (`.Stamina_14_5C277ACB4ABCD6EEC76DC68BACD236A7` (break `/Game/Blueprints/BlueprintComponents/S_Stats` (`self.Stats`))) 1.0)) ; Returns True if stamina is greater than 1
)

(fn `Sprinting`
  (params (StaminaDrain :type "Float (double-precision)" :default 2.0))
  (bind (_health _mana _savedlocation _gold _experience _stamina) (break `/Game/Blueprints/BlueprintComponents/S_Stats` (`self.Stats`)))
  (set `self.Stats` (make `/Game/Blueprints/BlueprintComponents/S_Stats` _health _mana _savedlocation _gold _experience (- _stamina StaminaDrain))))