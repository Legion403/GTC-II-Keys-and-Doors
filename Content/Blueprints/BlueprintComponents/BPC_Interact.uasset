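; Player interaction component for BP_FirstPersonCharacter that handles picking up, dropping, using and swapping held belt items.
; A self-restarting delayed loop sphere-traces from the camera to track the BPI_Interactable actor being looked at.
; Key presses send interface messages to items and update BPC_BeltInventory and its grid widget.
; Number keys or active-slot updates respawn the held actor from slot data; an older line-trace check is left unconnected.
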(event `self.ReceiveBeginPlay`
  (bind _asbp_first_person_character (cast `/Game/FirstPerson/Blueprints/BP_FirstPersonCharacter` (`self.GetOwner`)))
  (bind _output_get (set `self.As BP First Person Character` _asbp_first_person_character))
  (set `self.First Person Camera` (`/Game/FirstPerson/Blueprints/BP_FirstPersonCharacter.FirstPersonCamera` _output_get))
  (`self.Try to interact`)
  ; Spawn whatevers in slot 0
  (`self.Swap Active Item` 0)
  (add `/Game/Blueprints/BPC_Inventory.OnSlotUpdated` (`/Game/FirstPerson/Blueprints/BP_FirstPersonCharacter.BPC_BeltInventory` (`self.As BP First Person Character`)) (delegate `OnSlotUpdated_Event`)))

(event `OnSlotUpdated_Event`
  (params (Slot :type Integer))
  (`self.Update Held Item` Slot))

(event `Try to interact`
  (bind _first_person_camera (`self.First Person Camera`))
  (bind _returnvalue (`SceneComponent.K2_GetComponentLocation` _first_person_camera))
  (`KismetSystemLibrary.Delay` 0.4)
  (bind (_outhit _returnvalue_2) (`KismetSystemLibrary.SphereTraceSingle` :`Start` _returnvalue :`End` (+ _returnvalue (* (`SceneComponent.GetForwardVector` _first_person_camera) (`self.Look Distance`))) :`Radius` 50.0 :`TraceChannel` "TraceTypeQuery1" :`TraceColor` (struct :`R` 1.0 :`B` 0.298591 :`A` 0.196522) :`TraceHitColor` (struct :`G` 1.0 :`B` 0.441072 :`A` 1.0) :`DrawTime` 1.0))
  (if _returnvalue_2
    (bind (_bblockinghit _binitialoverlap _time _distance _location _impactpoint _normal _impactnormal _physmat _hitactor) (`GameplayStatics.BreakHitResult` _outhit))
    (if (`KismetSystemLibrary.DoesImplementInterface` _hitactor "/Game/Blueprints/BlueprintComponents/BPI_Interactable.BPI_Interactable_C")
      (set `self.LastTouchedItem` _hitactor)
      (else
        (set `self.LastTouchedItem` null)))
    (`self.Try to interact`)
    (else
      (set `self.LastTouchedItem` null)
      (`self.Try to interact`))))

(event `Key|Tab`
  (params (Key :type "Key Structure"))
  ; Interaction messages to interface
  (:`Pressed`
    (`self.Try to drop`)))

(event `Key|Enter`
  (params (Key :type "Key Structure"))
  ; Interaction messages to interface
  (:`Pressed`
    (`self.Try to pickup`)
    (`self.tRY TO ALT USE`)))

(event `Key|E`
  (params (Key :type "Key Structure"))
  ; Interaction messages to interface
  (:`Pressed`
    (`self.Try to pickup`)
    (`self.Try to Use`)))

(event `Try to drop`
  (bind _as_bp_first_person_character (`self.As BP First Person Character`))
  (bind _helditem (`self.HeldItem`))
  ; Interaction messages to interface
  (`Actor.K2_DetachFromActor` _helditem "KeepRelative" "KeepRelative" "KeepRelative")
  (message `/Game/Blueprints/BlueprintComponents/BPI_Interactable.Drop` _helditem)
  (`/Game/Blueprints/BPC_Inventory.Set Slot` (`/Game/FirstPerson/Blueprints/BP_FirstPersonCharacter.BPC_BeltInventory` _as_bp_first_person_character) "NewEnumerator4" (`self.Active Slott`))
  (`/Game/Widget/W_InventoryGrid.Refresh Grid` (`/Game/Widget/W_Belt.W_InventoryGrid` (`/Game/FirstPerson/Blueprints/BP_FirstPersonCharacter.BeltWidget` _as_bp_first_person_character))))

(event `Try to pickup`
  (bind _as_bp_first_person_character (`self.As BP First Person Character`))
  ; Interaction messages to interface
  (bind _lasttoucheditem (`self.LastTouchedItem`)
    (:`then`
      (bind _output_get (set `self.HeldItem` _lasttoucheditem))
      (bind _itemtype (message `/Game/Blueprints/BlueprintComponents/BPI_Interactable.PickUp` _output_get))
      (`/Game/Blueprints/BPC_Inventory.Set Slot` (`/Game/FirstPerson/Blueprints/BP_FirstPersonCharacter.BPC_BeltInventory` _as_bp_first_person_character) _itemtype (`self.Active Slott`))
      (`/Game/Widget/W_InventoryGrid.Refresh Grid` (`/Game/Widget/W_Belt.W_InventoryGrid` (`/Game/FirstPerson/Blueprints/BP_FirstPersonCharacter.BeltWidget` _as_bp_first_person_character))))
    (:`else`)))

(event `Try to Use`
  (bind _as_bp_first_person_character (`self.As BP First Person Character`))
  ; Interaction messages to interface
  (message `/Game/Blueprints/BlueprintComponents/BPI_Interactable.Use` (`self.HeldItem`))
  (if true
    (`/Game/Blueprints/BPC_Inventory.Set Slot` (`/Game/FirstPerson/Blueprints/BP_FirstPersonCharacter.BPC_BeltInventory` _as_bp_first_person_character) "NewEnumerator4" (`self.Active Slott`))
    (`/Game/Widget/W_InventoryGrid.Refresh Grid` (`/Game/Widget/W_Belt.W_InventoryGrid` (`/Game/FirstPerson/Blueprints/BP_FirstPersonCharacter.BeltWidget` _as_bp_first_person_character)))))

(event `tRY TO ALT USE`
  ; Interaction messages to interface
  (message `/Game/Blueprints/BlueprintComponents/BPI_Interactable.AltUse` (`self.HeldItem`)))

(event `Key|One`
  (params (Key :type "Key Structure"))
  (:`Pressed`
    (`self.Swap Active Item` 0)))

(event `Key|Two`
  (params (Key :type "Key Structure"))
  (:`Pressed`
    (`self.Swap Active Item` 1)))

(event `Key|Three`
  (params (Key :type "Key Structure"))
  (:`Pressed`
    (`self.Swap Active Item` 2)))

(event `Key|Four`
  (params (Key :type "Key Structure"))
  (:`Pressed`
    (`self.Swap Active Item` 3)))

(event `Swap Active Item`
  (params (`New Slot Index` :type Integer))
  (bind _as_bp_first_person_character (`self.As BP First Person Character`))
  (bind (_name _description _ui_image _actorbp _autopickupable _enum) (break `/Game/Blueprints/S_item` (`/Game/Blueprints/BPC_Inventory.Get Slot` (`/Game/FirstPerson/Blueprints/BP_FirstPersonCharacter.BPC_BeltInventory` _as_bp_first_person_character) `New Slot Index`)))
  ; Swap
  (if (!= `New Slot Index` (`self.Active Slott`))
    (set `self.Active Slott` `New Slot Index`)
    (`self.HeldItem` :!label _label
      (:`then`
        (`Actor.K2_DestroyActor` (`self.HeldItem`)))
      (:`else`
        _))
    (if (`|EnumInequality` _enum "NewEnumerator4")
      (bind _returnvalue (`|SpawnActorFromClass` _actorbp (`KismetMathLibrary.Conv_VectorToTransform` (`SceneComponent.GetSocketLocation` (`/Game/FirstPerson/Blueprints/BP_FirstPersonCharacter.Socket` _as_bp_first_person_character) "None")) "Undefined" "MultiplyWithRoot" null null))
      (bind _output_get (set `self.HeldItem` _returnvalue))
      (message `/Game/Blueprints/BlueprintComponents/BPI_Interactable.PickUp` _output_get)
      (else
        (`Actor.K2_DestroyActor` (`self.HeldItem`))
        (set `self.Held Item` null)))))

(event `Update Held Item`
  (params (`Newly changed slot` :type Integer))
  (if (== (`self.Active Slott`) `Newly changed slot`)
    (goto _label)))