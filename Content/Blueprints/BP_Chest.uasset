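; BP_Chest is a chest actor with an inventory component that opens when the first-person character enters its trigger box.
; Overlap plays the lid montage, prints debug text, shows a chest menu created at BeginPlay and opens the character's chest inventory view.
; On opening, it registers the inventory with the GM_SaveLoad game mode's level state, and LoadSavedInventory restores the saved EnumInventory.
; Leaving the box removes the menu.
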(event `self.ReceiveBeginPlay`
  (bind _returnvalue (`|CreateWidget` "/Game/Widget/W_ChestMenu.W_ChestMenu_C" null (`self.BPC_Inventory`)))
  (set `self.ChestMenu` _returnvalue))

(event `self.Box.OnComponentBeginOverlap`
  (params (OverlappedComponent :type "PrimitiveComponent Object Reference") (OtherActor :type "Actor Object Reference") (OtherComp :type "PrimitiveComponent Object Reference") (OtherBodyIndex :type Integer) (bFromSweep :type Boolean) (SweepResult :type "HitResult Structure (by ref)"))
  (bind _asbp_first_person_character (cast `/Game/FirstPerson/Blueprints/BP_FirstPersonCharacter` OtherActor))
  (set `self.As BP First Person Character` _asbp_first_person_character)
  (`SkeletalMeshComponent.PlayAnimation` (`self.BasicChestLid`) "/Game/3DObjects/BasicChestLid/SkeletalMeshes/BasicChestLid_Anim_Montage.BasicChestLid_Anim_Montage" false)
  (`KismetSystemLibrary.PrintText` (`|FormatText` "First item is a {Name}" (`.Name_4_6AC0ECD843F1213FB77D3BB15E103619` (break `/Game/Blueprints/S_item` (`|GetArrayItem` (`/Game/Blueprints/BPC_Inventory.Inventory` (`self.BPC_Inventory`)))))))
  (`KismetSystemLibrary.PrintString` "Opened Chest!")
  (`UserWidget.AddToViewport` (`self.ChestMenu`) 0)
  (`/Game/FirstPerson/Blueprints/BP_FirstPersonCharacter.Chest Open Inventory` (`self.As BP First Person Character`))
  ; Saving the inventory to load later
  (bind _asgm_save_load (cast `/Game/Blueprints/GM_SaveLoad` (`GameplayStatics.GetGameMode`)))
  (`/Game/Blueprints/SaveLoad/SG_levelstate.Add Inventory` (`/Game/Blueprints/GM_SaveLoad.LevelState` _asgm_save_load) (`self.BPC_Inventory`)))

(event `self.Box.OnComponentEndOverlap`
  (params (OverlappedComponent :type "PrimitiveComponent Object Reference") (OtherActor :type "Actor Object Reference") (OtherComp :type "PrimitiveComponent Object Reference") (OtherBodyIndex :type Integer))
  (cast `/Game/FirstPerson/Blueprints/BP_FirstPersonCharacter` OtherActor)
  (`Widget.RemoveFromParent` (`self.ChestMenu`)))

(event `Load Saved Inventory`
  (params (EnumInventory :type "Array of /Game/Blueprints/E_Item Enum"))
  (set `/Game/Blueprints/BPC_Inventory.EnumInventory` EnumInventory (`self.BPC_Inventory`)) ; Replace current inventory with our saved inventory
)

(fn `UserConstructionScript`)