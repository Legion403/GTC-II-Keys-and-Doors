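; Inventory component that stores the player's items as an array of item enums, one per slot.
; Slot reads resolve the enum to full item data by scanning DT_Items rows for a matching Enum field.
; Setting a slot fires a slot-updated dispatcher, while replacing the whole array fires a grid-refresh dispatcher so listeners such as UI can update.
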(fn `Get Item Details`
  (params (`Requested Item` :type "/Game/Blueprints/E_Item Enum" :default "NewEnumerator0"))
  (returns (`Item Details` :type "/Game/Blueprints/S_item Structure"))
  (bind _outrownames (`DataTableFunctionLibrary.GetDataTableRowNames` "/Game/Blueprints/DataTables/DT_Items.DT_Items"))
  (for _array_element _outrownames
    (bind _returnvalue (`|GetDataTableRow` "/Game/Blueprints/DataTables/DT_Items.DT_Items" _array_element)
      (:`then`
        (if (`|EnumEquality` (`.Enum_19_44267B1F4286AEA37A2AF794615BB42B` (break `/Game/Blueprints/S_item` _returnvalue)) `Requested Item`)
          (return _returnvalue))))))

(fn `Get Slot`
  (params (`Requested Slot` :type Integer))
  (returns (ItemDetails :type "/Game/Blueprints/S_item Structure"))
  (bind _item_details (`self.Get Item Details` (`|GetArrayItem` (`self.EnumInventory`) `Requested Slot`)))
  (return _item_details))

(fn `Set Slot`
  (params (ItemEnum :type "/Game/Blueprints/E_Item Enum" :default "NewEnumerator0") (SlotNumber :type Integer))
  (`KismetArrayLibrary.Array_Set` (`self.EnumInventory`) SlotNumber ItemEnum)
  (`self.OnSlotUpdated` SlotNumber))

(fn `SetEnumArray`
  (params (EnumInventory :type "Array of /Game/Blueprints/E_Item Enum"))
  (set `self.EnumInventory` EnumInventory)
  (`self.OnEventRefreshGrid`))