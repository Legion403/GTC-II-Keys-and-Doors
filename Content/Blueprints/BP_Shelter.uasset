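; BP_Shelter is a destructible shelter actor that loses health only from damage of the exact type BP_PlayerDamage.
; Each hit lowers a clamped CurrentHealth and sets IsDead when it reaches zero.
; A subsequent player hit, not the lethal one, triggers a DoOnce that spawns a Niagara explosion at the WallNoEdges component and destroys the actor after a short delay.
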(event `self.ReceiveAnyDamage`
  (params (Damage :type "Float (single-precision)") (DamageType :type "DamageType Object Reference") (InstigatedBy :type "Controller Object Reference") (DamageCauser :type "Actor Object Reference"))
  (if (== (`GameplayStatics.GetObjectClass` DamageType) "/Game/FirstPerson/Blueprints/HealthAndDamage/BP_PlayerDamage.BP_PlayerDamage_C")
    (if (`self.IsDead`)
      (`/Engine/EditorBlueprintResources/StandardMacros.DoOnce` false
        (:`Completed`
          (`NiagaraFunctionLibrary.SpawnSystemAtLocation` "/Game/VFX/ExplosionVFX/NS_Explosion.NS_Explosion" (`SceneComponent.K2_GetComponentLocation` (`self.WallNoEdges`)))
          (`KismetSystemLibrary.Delay` 1.0)
          (`self.K2_DestroyActor`)))
      (else
        (bind _output_get (set `self.CurrentHealth` (`KismetMathLibrary.FClamp` (- (`self.CurrentHealth`) Damage) 0.0 (`self.Max Health`))))
        (if (== _output_get 0.0)
          (set `self.IsDead` true))))))

(fn `UserConstructionScript`)