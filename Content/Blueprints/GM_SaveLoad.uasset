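; Game mode that saves and loads player progress and per-level state.
; On BeginPlay it loads existing saves or creates SG_Player (belt and inventory, in SlotName) and SG_levelstate (player transform, in a slot named after the level).
; Load refills the character's inventory components, calls ActivateActors on the level state and restores position and view rotation.
; Delete functions clear both slots or only the level's, then reopen the level.
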(event `self.ReceiveBeginPlay`
  (`KismetSystemLibrary.PrintString` "starting gm save/load")
  (`|ExecutionSequence`
    (:`then_0`
      (bind _returnvalue (`GameplayStatics.DoesSaveGameExist` (`self.Slot Name`)))
      (if _returnvalue
        (`self.Load`)
        (else
          (bind _returnvalue_2 (`GameplayStatics.CreateSaveGameObject` "/Game/Blueprints/SG_Player.SG_Player_C"))
          (set `self.PlayerSave` _returnvalue_2))))
    (:`then_1`
      (bind _returnvalue_3 (`GameplayStatics.GetCurrentLevelName` true))
      (bind _returnvalue_4 (`GameplayStatics.DoesSaveGameExist` _returnvalue_3))
      (if _returnvalue_4
        (`self.Load`)
        (else
          (bind _returnvalue_5 (`GameplayStatics.CreateSaveGameObject` "/Game/Blueprints/SaveLoad/SG_levelstate.SG_levelstate_C"))
          (set `self.LevelState` _returnvalue_5))))))

(fn `Delete Level Save`
  (bind _returnvalue (`GameplayStatics.GetCurrentLevelName` true))
  (`GameplayStatics.DeleteGameInSlot` _returnvalue)
  (`GameplayStatics.OpenLevel` (`KismetStringLibrary.Conv_StringToName` _returnvalue)))

(fn `Delete Save`
  (`GameplayStatics.DeleteGameInSlot` (`self.Slot Name`))
  (`self.Delete Level Save`))

(fn `Load`
  (bind _playertransform (`/Game/Blueprints/SaveLoad/SG_levelstate.PlayerTransform` (`self.LevelState`)))
  (`|ExecutionSequence`
    (:`then_0`
      (bind _returnvalue (`GameplayStatics.LoadGameFromSlot` (`self.Slot Name`)))
      (bind _assg_player (cast `/Game/Blueprints/SG_Player` _returnvalue))
      (bind _output_get (set `self.PlayerSave` _assg_player))
      (bind _asbp_first_person_character (cast `/Game/FirstPerson/Blueprints/BP_FirstPersonCharacter` (`GameplayStatics.GetPlayerCharacter` 0)))
      (`/Game/Blueprints/BPC_Inventory.SetEnumArray` (`/Game/FirstPerson/Blueprints/BP_FirstPersonCharacter.BPC_BeltInventory` _asbp_first_person_character) (`/Game/Blueprints/SG_Player.Belt` _output_get))
      (`/Game/Blueprints/BPC_Inventory.SetEnumArray` (`/Game/FirstPerson/Blueprints/BP_FirstPersonCharacter.BPC_Inventory` _asbp_first_person_character) (`/Game/Blueprints/SG_Player.PlayerInv` _output_get))
      (`/Game/FirstPerson/Blueprints/BP_FirstPersonCharacter.Load transform` _asbp_first_person_character (`/Game/Blueprints/SaveLoad/SG_levelstate.PlayerTransform` (`self.LevelState`)) (0.0 0.0 0.0)) ; Moving the player to the last saved position
    )
    (:`then_1`
      (bind _returnvalue_2 (`GameplayStatics.GetCurrentLevelName` true))
      (bind _returnvalue_3 (`GameplayStatics.LoadGameFromSlot` _returnvalue_2))
      (bind _assg_levelstate (cast `/Game/Blueprints/SaveLoad/SG_levelstate` _returnvalue_3))
      (bind _output_get_2 (set `self.LevelState` _assg_levelstate))
      (`/Game/Blueprints/SaveLoad/SG_levelstate.ActivateActors` _output_get_2)
      (bind _asbp_first_person_character_2 (cast `/Game/FirstPerson/Blueprints/BP_FirstPersonCharacter` (`GameplayStatics.GetPlayerCharacter` 0)))
      (`/Game/FirstPerson/Blueprints/BP_FirstPersonCharacter.Load transform` _asbp_first_person_character_2 _playertransform (0.0 0.0 0.0))
      (`Controller.SetControlRotation` (`GameplayStatics.GetPlayerController` 0) (.rotation _playertransform)))))

(fn `Save`
  (params (Belt :type "Array of /Game/Blueprints/E_Item Enum") (PlayerInv :type "Array of /Game/Blueprints/E_Item Enum") (`Player Transform` :type "Transform Structure"))
  (bind _playersave (`self.PlayerSave`))
  (`|ExecutionSequence`
    (:`then_0`
      ; Player stuff to save
      (set `/Game/Blueprints/SG_Player.Belt` Belt _playersave)
      (set `/Game/Blueprints/SG_Player.PlayerInv` PlayerInv _playersave)
      (`GameplayStatics.SaveGameToSlot` (`self.PlayerSave`) (`self.Slot Name`)))
    (:`then_1`
      (set `/Game/Blueprints/SaveLoad/SG_levelstate.PlayerTransform` `Player Transform` (`self.LevelState`))
      ; level state to save
      (bind _returnvalue (`GameplayStatics.GetCurrentLevelName` true))
      (`GameplayStatics.SaveGameToSlot` (`self.LevelState`) _returnvalue))))

(fn `UserConstructionScript`)