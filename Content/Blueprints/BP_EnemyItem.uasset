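; Pickup item, built around a Key component, that spawns a BP_Enemy when used.
; PickUp sets HasKey on the first-person character, then once plays a coin sound, attaches the item to the character's socket after a short delay, animates the key and disables collision.
; Use spawns the enemy at the player camera's transform and destroys the item.
; Drop and AltUse are empty, and a camera line trace is left unconnected.
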(event `self.ReceiveBeginPlay`
  (bind _asbp_first_person_character (cast `/Game/FirstPerson/Blueprints/BP_FirstPersonCharacter` (`GameplayStatics.GetPlayerCharacter` 0)))
  (set `self.As BP First Person Character` _asbp_first_person_character))

(event `self.PickUp`
  (set `/Game/FirstPerson/Blueprints/BP_FirstPersonCharacter.HasKey` true (`self.As BP First Person Character`))
  (`/Engine/EditorBlueprintResources/StandardMacros.DoOnce` false
    (:`Completed`
      (`GameplayStatics.PlaySound2D` "/Game/SoundEffects/573374__doudar41__coins35.573374__doudar41__coins35" 1.0 1.0 0.0 null null)
      (`KismetSystemLibrary.Delay` 0.2)
      (`self.K2_AttachToComponent` (`/Game/FirstPerson/Blueprints/BP_FirstPersonCharacter.Socket` (`self.As BP First Person Character`)) "None" "SnapToTarget" "SnapToTarget" "KeepRelative")
      (`SkeletalMeshComponent.PlayAnimation` (`self.Key`) null false)
      (`PrimitiveComponent.SetCollisionEnabled` (`self.Key`) "NoCollision")
      (`PrimitiveComponent.SetCollisionEnabled` (`self.Sphere`) "NoCollision"))))

(event `self.Drop`)

(event `self.Use`
  (`|SpawnActorFromClass` "/Game/AI/BP_Enemy.BP_Enemy_C" (`KismetMathLibrary.Conv_VectorToTransform` (`SceneComponent.GetSocketLocation` (`/Game/FirstPerson/Blueprints/BP_FirstPersonCharacter.FirstPersonCamera` (`self.As BP First Person Character`)) "None")) "Undefined" "MultiplyWithRoot" null null)
  (`self.K2_DestroyActor`))

(event `self.AltUse`)

(fn `UserConstructionScript`)