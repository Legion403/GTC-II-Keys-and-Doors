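; BP_MusicHandler runs a Quartz metronome that plays beep sounds on bars and beats at a given BPM.
; StartNewClock creates a 4/4 "MusicClock", sets its tempo, prepares two 2D MetaSound beeps and subscribes to all quantization events.
; The quantization handler queues the A4 beep on Bar events and the A3 beep on Beat events, using PlayQuantized for clock-aligned playback.
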(event `StartNewClock`
  (params (BPM :type "Float (double-precision)"))
  (bind _returnvalue (`QuartzSubsystem.CreateNewClock` (subsystem `QuartzSubsystem`) "MusicClock" (make `QuartzClockSettings` (make `QuartzTimeSignature` 4)) false true))
  (bind _output_get (set `self.ClockHandel` _returnvalue))
  (bind _clockhandle (`QuartzClockHandle.StartClock` _output_get))
  (`QuartzClockHandle.SetBeatsPerMinute` :`self` _clockhandle :`BeatsPerMinute` BPM)
  (bind _returnvalue_2 (`GameplayStatics.CreateSound2D` "/Game/Blueprints/Quartz/MSS_BeepA4.MSS_BeepA4" 1.0 1.0 0.0 null))
  (bind _output_get_2 (set `self.MSS_BEEPA4` _returnvalue_2))
  (set `AudioComponent.bCanPlayMultipleInstances` true _output_get_2)
  (bind _returnvalue_3 (`GameplayStatics.CreateSound2D` "/Game/Blueprints/Quartz/MSS_BeepA3.MSS_BeepA3" 1.0 1.0 0.0 null))
  (bind _output_get_3 (set `self.MSS_BEEPA3` _returnvalue_3))
  (set `AudioComponent.bCanPlayMultipleInstances` true _output_get_3)
  (bind _clockhandle_2 (`QuartzClockHandle.StartClock` (`self.ClockHandel`)))
  (`QuartzClockHandle.SubscribeToAllQuantizationEvents` _clockhandle_2 (`|CreateDelegate` :!event `OnQuantizationEvent`)))

(event `OnQuantizationEvent`
  (params (ClockName :type Name) (QuantizationType :type "EQuartzCommandQuantization Enum" :default "Bar") (NumBars :type Integer) (Beat :type Integer) (BeatFraction :type "Float (single-precision)"))
  (switch `EQuartzCommandQuantization` QuantizationType
    (:`Bar`
      (`AudioComponent.PlayQuantized` :`self` (`self.MSS_BEEPA4`) :`InClockHandle` (`self.ClockHandel`) :`InQuantizationBoundary` (make `QuartzQuantizationBoundary` QuantizationType 1.0 "TransportRelative")))
    (:`Beat`
      (`AudioComponent.PlayQuantized` :`self` (`self.MSS_BEEPA3`) :`InClockHandle` (`self.ClockHandel`) :`InQuantizationBoundary` (make `QuartzQuantizationBoundary` QuantizationType 1.0 "TransportRelative")))))

(fn `UserConstructionScript`)