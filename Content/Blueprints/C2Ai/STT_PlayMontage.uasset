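; StateTree task that plays a montage on an AI character and performs its attack as the montage starts.
; A forward sphere trace with debug drawing runs, then a cast to BP_RangedEnemy gates both ShootFireball and enemy damage to any traced hit.
; The task succeeds when the montage completes and fails when it is interrupted.
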(event `self.ReceiveLatentEnterState`
  (params (Transition :type "StateTreeTransitionResult Structure (by ref)"))
  (bind _character (`self.Character`))
  (bind _returnvalue (`Actor.K2_GetActorLocation` _character))
  (`|PlayMontage` (`Character.Mesh` (`self.Character`)) (`self.Montage to Play`)
    (:`then`
      (bind (_outhit _returnvalue_2) (`KismetSystemLibrary.SphereTraceSingle` _returnvalue (+ _returnvalue (* (`Actor.GetActorForwardVector` _character) 150.0)) 50.0 "TraceTypeQuery2" false (`|MakeArray` (`self.Character`) :!type "Actor Object Reference") "ForDuration" true (struct :`R` 1.0 :`A` 1.0) (struct :`G` 1.0 :`A` 1.0) 3.0))
      (bind _asbp_ranged_enemy (cast `/Game/Blueprints/C2Ai/BP_RangedEnemy` (`self.Character`)))
      (`KismetSystemLibrary.PrintString` "LIFTING!")
      (`/Game/Blueprints/C2Ai/BP_RangedEnemy.ShootFireball` _asbp_ranged_enemy)
      (if _returnvalue_2
        (`GameplayStatics.ApplyDamage` (`.HitActor` (`GameplayStatics.BreakHitResult` _outhit)) 25.0 null null "/Game/FirstPerson/Blueprints/HealthAndDamage/BP_EnemyDamage.BP_EnemyDamage_C")))
    (:`OnCompleted`
      (`self.FinishTask` true))
    (:`OnInterrupted`
      (`self.FinishTask` false))))