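; BP_NewSecurityCamera is a security camera that alerts AI when a target is sighted.
; HandleSight takes a sensing result; on success it swaps the static mesh to a godray material and plays a sound at the camera.
; It then gets every BP_DummyAi in the level and sends each to check out the alarm at StimulusLocation.
; Losing the target switches the mesh to the laser pointer material.
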(fn `HandleSight`
  (params (Target :type "Actor Object Reference") (SuccessfullySensed :type Boolean))
  (if SuccessfullySensed
    (`KismetSystemLibrary.PrintText` "Acuired Target")
    (`PrimitiveComponent.SetMaterial` (`self.StaticMesh`) 0 "/Game/VFX/Materials/MM_Godray_Inst.MM_Godray_Inst")
    (`GameplayStatics.PlaySoundAtLocation` "/Game/SoundEffects/diablo_2_portal.diablo_2_portal" (`self.K2_GetActorLocation`) (struct) 2.0 1.0 0.0 "/Game/SoundEffects/Attenuation/DefaultAttenuation.DefaultAttenuation" null null null)
    (bind _outactors (`GameplayStatics.GetAllActorsOfClass` "/Game/Blueprints/C2Ai/BP_DummyAi.BP_DummyAi_C"))
    (for _array_element _outactors
      (`/Game/Blueprints/C2Ai/BP_DummyAi.CheckOutSecurityAlarm` _array_element (`self.Stimulus Location`)))
    (else
      (`KismetSystemLibrary.PrintText` "Lost target")
      (`PrimitiveComponent.SetMaterial` (`self.StaticMesh`) 0 "/Engine/VREditor/LaserPointer/LaserPointerMaterial.LaserPointerMaterial"))))

(fn `UserConstructionScript`)