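; BP_RangedEnemy is an AI-controlled ranged enemy that fires projectiles, takes player damage and leaves a soul on death.
; ShootFireball spawns both a fireball and an enemy projectile at the Fireball component.
; Damage is reported to perception and sent to AIC_Basic's StateTree, but only BP_PlayerDamage reduces health.
; Zero health sets IsDead; the next player hit triggers the flame burst, soul spawn and destruction.
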(event `self.ReceiveBeginPlay`
  (bind _asaic_basic (cast `/Game/Blueprints/C2Ai/AIC_Basic` (`self.GetController`)))
  (set `self.As AIC Basic` _asaic_basic))

(event `ShootFireball`
  (bind _returnvalue (`SceneComponent.K2_GetComponentToWorld` (`self.Fireball`)))
  (`|SpawnActorFromClass` "/Game/FirstPerson/Blueprints/HealthAndDamage/Projectiles/BP_FireballProjEnemy.BP_FireballProjEnemy_C" _returnvalue "Undefined" "MultiplyWithRoot" null null)
  (`|SpawnActorFromClass` "/Game/Blueprints/BP_EnemyProjectile.BP_EnemyProjectile_C" _returnvalue "Undefined" "MultiplyWithRoot" null null))

(event `self.ReceiveAnyDamage`
  (params (Damage :type "Float (single-precision)") (DamageType :type "DamageType Object Reference") (InstigatedBy :type "Controller Object Reference") (DamageCauser :type "Actor Object Reference"))
  (bind _returnvalue (`self.K2_GetActorLocation`))
  (`AISense_Damage.ReportDamageEvent` self InstigatedBy Damage (`self.K2_GetActorLocation` (`Controller.K2_GetPawn` InstigatedBy))) ; Not working?
  ; Death and Health
  (`StateTreeComponent.SendStateTreeEvent` (`/Game/Blueprints/C2Ai/AIC_Basic.StateTreeAI` (`self.As AIC Basic`)) (make `StateTreeEvent` (struct :`TagName` "AI.Event.TookDamage")))
  (if (== (`GameplayStatics.GetObjectClass` DamageType) "/Game/FirstPerson/Blueprints/HealthAndDamage/BP_PlayerDamage.BP_PlayerDamage_C")
    (if (`self.IsDead`)
      (`NiagaraFunctionLibrary.SpawnSystemAtLocation` "/Game/VFX/NS_FlameBurst.NS_FlameBurst" _returnvalue)
      (`KismetSystemLibrary.Delay` 0.2)
      (`|SpawnActorFromClass` "/Game/Blueprints/BP_Soul.BP_Soul_C" (`KismetMathLibrary.Conv_VectorToTransform` _returnvalue) "Undefined" "MultiplyWithRoot" null null)
      (`self.K2_DestroyActor`)
      (else
        (bind _output_get (set `self.CurrentHealth` (`KismetMathLibrary.FClamp` (- (`self.CurrentHealth`) Damage) 0.0 (`self.MaxHealth`))))
        (if (== _output_get 0.0)
          (set `self.IsDead` true))))))

(event `Get medkit`
  (params (`Health to add` :type "Float (double-precision)"))
  (bind _output_get (set `self.CurrentHealth` (`KismetMathLibrary.FClamp` (+ `Health to add` (`self.CurrentHealth`)) 0.0 50.0)))
  (`KismetSystemLibrary.PrintString` (`KismetStringLibrary.Conv_DoubleToString` _output_get)))

(fn `UserConstructionScript`)