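; BP_SecurityCamera is a security camera that raises an alarm when its AI Perception sees a target.
; Perception updates store the stimulus location, skip sight handling for AI-tagged stimuli and route other sight stimuli to HandleSight.
; On detection it swaps its mesh material, plays a sound and sends every BP_DummyAi to check out that location.
; Losing sight swaps to the laser pointer material, with debug prints throughout.
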(event `self.AIPerception.OnTargetPerceptionUpdated`
  (params (Actor :type "Actor Object Reference") (Stimulus :type "AIStimulus Structure"))
  (bind (_age _expirationage _strength _stimuluslocation _receiverlocation _tag _bsuccessfullysensed) (break `AIStimulus` Stimulus))
  (bind _returnvalue (`AIPerceptionSystem.GetSenseClassForStimulus` Stimulus))
  (set `self.Stimulus Location` _stimuluslocation)
  (bind _returnvalue_2 (`KismetSystemLibrary.GetClassDisplayName` _returnvalue))
  (`KismetSystemLibrary.PrintString` (`KismetTextLibrary.Conv_TextToString` (`|FormatText` "Sensed: {actor} with {name}" Actor (`KismetTextLibrary.Conv_StringToText` _returnvalue_2))))
  (switch `name` _tag
    (:`Default`
      (switch `string` _returnvalue_2
        (:`AISense_Sight`
          (`self.HandleSight` Actor _bsuccessfullysensed))))
    (:`AI`
      (`KismetSystemLibrary.PrintString` "Hello Friend"))))

(event `self.AIPerception.OnTargetPerceptionForgotten`
  (params (Actor :type "Actor Object Reference"))
  (`KismetSystemLibrary.PrintText` (`|FormatText` "Forgot {actor}!" Actor)))

(event `self.AIPerception.OnTargetPerceptionInfoUpdated`
  (params (UpdateInfo :type "ActorPerceptionUpdateInfo Structure (by ref)")))

(fn `HandleSight`
  (params (Target :type "Actor Object Reference") (SuccessfullySensed :type Boolean))
  (if SuccessfullySensed
    (`KismetSystemLibrary.PrintText` "Acuired Target")
    (`PrimitiveComponent.SetMaterial` (`self.StaticMesh`) 0 "/Game/VFX/Materials/MM_Godray_Inst.MM_Godray_Inst")
    (`GameplayStatics.PlaySoundAtLocation` "/Game/SoundEffects/diablo_2_portal.diablo_2_portal" (`self.K2_GetActorLocation`) (struct) 2.0 1.0 0.0 "/Game/SoundEffects/Attenuation/DefaultAttenuation.DefaultAttenuation" null null null)
    (bind _outactors (`GameplayStatics.GetAllActorsOfClass` "/Game/Blueprints/C2Ai/BP_DummyAi.BP_DummyAi_C"))
    (for _array_element _outactors
      (`/Game/Blueprints/C2Ai/BP_DummyAi.CheckOutSecurityAlarm` _array_element (`self.Stimulus Location`)))
    (else
      (`KismetSystemLibrary.PrintText` "Lost target")
      (`PrimitiveComponent.SetMaterial` (`self.StaticMesh`) 0 "/Engine/VREditor/LaserPointer/LaserPointerMaterial.LaserPointerMaterial"))))

(fn `UserConstructionScript`)