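; AI controller for security cameras and turrets that reacts to what its AI Perception senses.
; On possess it caches the pawn as camera or turret, and perception updates skip actors tagged AI and route sight stimuli to HandleSight.
; HandleSight forwards the sensed state to the camera; its turret branch calls HandleSight with the turret as Target.
; Debug prints report sensed and forgotten actors, and leftover alarm logic is never run.
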(event `self.ReceivePossess`
  (params (PossessedPawn :type "Pawn Object Reference"))
  (bind _asbp_new_security_camera (cast `/Game/Blueprints/C2Ai/BP_NewSecurityCamera` PossessedPawn)
    (:`then`
      (set `self.As BP New Security Camera` _asbp_new_security_camera))
    (:`CastFailed`
      (bind _asbp_turret (cast `/Game/Blueprints/C2Ai/BP_Turret` PossessedPawn))
      (set `self.As BP Turret` _asbp_turret))))

(event `self.AIPerception.OnTargetPerceptionUpdated`
  (params (Actor :type "Actor Object Reference") (Stimulus :type "AIStimulus Structure"))
  (bind (_age _expirationage _strength _stimuluslocation _receiverlocation _tag _bsuccessfullysensed) (break `AIStimulus` Stimulus))
  (if (not (`self.ActorHasTag` Actor "AI"))
    (bind _returnvalue (`AIPerceptionSystem.GetSenseClassForStimulus` Stimulus))
    (set `self.Stimulus Location` _stimuluslocation)
    (bind _returnvalue_2 (`KismetSystemLibrary.GetClassDisplayName` _returnvalue))
    (`KismetSystemLibrary.PrintString` (`KismetTextLibrary.Conv_TextToString` (`|FormatText` "Sensed: {actor} with {name}" Actor (`KismetTextLibrary.Conv_StringToText` _returnvalue_2))))
    (switch `name` _tag
      (:`Default`
        (switch `string` _returnvalue_2
          (:`AISense_Sight`
            (`self.HandleSight` Actor _bsuccessfullysensed))))
      (:`AI`
        (`KismetSystemLibrary.PrintString` "Hello Friend")))))

(event `self.AIPerception.OnTargetPerceptionForgotten`
  (params (Actor :type "Actor Object Reference"))
  (`KismetSystemLibrary.PrintText` (`|FormatText` "Forgot {actor}!" Actor)))

(event `self.AIPerception.OnTargetPerceptionInfoUpdated`
  (params (UpdateInfo :type "ActorPerceptionUpdateInfo Structure (by ref)")))

(fn `HandleSight`
  (params (Target :type "Actor Object Reference") (SuccessfullySensed :type Boolean))
  (bind _as_bp_new_security_camera (`self.As BP New Security Camera`)
    (:`then`
      (`/Game/Blueprints/C2Ai/BP_NewSecurityCamera.HandleSight` _as_bp_new_security_camera null SuccessfullySensed))
    (:`else`
      (bind _as_bp_turret (`self.As BP Turret`)
        (:`then`
          (`self.HandleSight` _as_bp_turret SuccessfullySensed))
        (:`else`)))))

(fn `UserConstructionScript`)