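; BP_Turret is an AI turret that tracks a sighted target and can fire physics-driven bullets.
; HandleSight stores a sensed target and switches to Tracking, or to Looking when sight fails.
; While tracking, Tick snaps rotation along the target-to-turret direction, so the actor's forward axis points away from the target.
; Attacking spawns BP_Bullet at BulletSpawn with a forward impulse, but nothing here calls it.
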(event `self.ReceiveBeginPlay`)

(event `self.ReceiveTick`
  (params (DeltaSeconds :type "Float (single-precision)"))
  (if (`self.TrackingTarget`)
    (`self.K2_SetActorRotation` (`KismetMathLibrary.FindLookAtRotation` (`self.K2_GetActorLocation` (`self.Target`)) (`self.K2_GetActorLocation`)))))

(event `Fire Projectile`
  (bind _bulletspawn (`self.BulletSpawn`))
  (bind _returnvalue (`|SpawnActorFromClass` "/Game/Blueprints/C2Ai/BP_Bullet.BP_Bullet_C" (`SceneComponent.K2_GetComponentToWorld` _bulletspawn) "Undefined" "MultiplyWithRoot" null null))
  (`PrimitiveComponent.AddImpulse` (`/Game/Blueprints/C2Ai/BP_Bullet.Cube` _returnvalue) (* (`SceneComponent.GetForwardVector` _bulletspawn) 3000.0) "None" false))

(event `Handle Sight`
  (params (Target :type "Actor Object Reference") (`Successfully Senesed` :type Boolean))
  (if `Successfully Senesed`
    (set `self.Target` Target)
    (`self.Tracking`)
    (else
      (`self.Looking`))))

(event `Looking`
  (set `self.TrackingTarget` false))

(event `Tracking`
  (set `self.TrackingTarget` true))

(event `Attacking`
  (`self.Fire Projectile`)
  (`self.Tracking`))

(fn `UserConstructionScript`)