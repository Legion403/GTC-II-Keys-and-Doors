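; BP_Nuke is a carryable bomb item that the player can detonate or use to open a door.
; PickUp sets the player's HasKey flag, plays a sound, attaches to the character's socket, disables sphere collision and returns its ItemType.
; Use spawns a big Niagara explosion at the bomb, while AltUse line-traces from the camera to open a BP_Door with an explosion.
; Both destroy the actor after a short delay; Drop is empty.
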(event `self.ReceiveBeginPlay`
  (bind _asbp_first_person_character (cast `/Game/FirstPerson/Blueprints/BP_FirstPersonCharacter` (`GameplayStatics.GetPlayerCharacter` 0)))
  (set `self.As BP First Person Character` _asbp_first_person_character))

(event `self.Drop`)

(event `self.AltUse`
  (bind _firstpersoncamera (`/Game/FirstPerson/Blueprints/BP_FirstPersonCharacter.FirstPersonCamera` (`self.As BP First Person Character`)))
  (bind _returnvalue (`SceneComponent.K2_GetComponentLocation` _firstpersoncamera))
  (bind (_outhit _returnvalue_2) (`KismetSystemLibrary.LineTraceSingle` (+ _returnvalue 1.0) (+ _returnvalue (* (`SceneComponent.GetForwardVector` _firstpersoncamera) (`self.LookDistance`))) "TraceTypeQuery1"))
  (if _returnvalue_2
    (bind _asbp_door (cast `/Game/Blueprints/BP_Door` (`.HitActor` (`GameplayStatics.BreakHitResult` _outhit))))
    (`/Game/Blueprints/BP_Door.Open Door` _asbp_door)
    (`NiagaraFunctionLibrary.SpawnSystemAtLocation` "/Game/VFX/ExplosionVFX/NS_Explosion.NS_Explosion" (`self.K2_GetActorLocation` _asbp_door))
    (`KismetSystemLibrary.Delay` 0.2)
    (`self.K2_DestroyActor`)))

(event `self.Use`
  (`NiagaraFunctionLibrary.SpawnSystemAtLocation` "/Game/VFX/ExplosionVFX/NS_BIGExplosion1.NS_BIGExplosion1" (`SceneComponent.K2_GetComponentLocation` (`self.Bomb`)))
  (`KismetSystemLibrary.Delay` 0.2)
  (`self.K2_DestroyActor`))

(fn `PickUp`
  (returns (ItemType :type "/Game/Blueprints/E_Item Enum"))
  (set `/Game/FirstPerson/Blueprints/BP_FirstPersonCharacter.HasKey` true (`self.As BP First Person Character`))
  (`/Engine/EditorBlueprintResources/StandardMacros.DoOnce` false
    (:`Completed`
      (`GameplayStatics.PlaySound2D` "/Game/SoundEffects/573374__doudar41__coins35.573374__doudar41__coins35" 1.0 1.0 0.0 null null)
      (`self.K2_AttachToComponent` (`/Game/FirstPerson/Blueprints/BP_FirstPersonCharacter.Socket` (`self.As BP First Person Character`)) "None" "SnapToTarget" "SnapToTarget" "KeepRelative")
      (`PrimitiveComponent.SetCollisionEnabled` (`self.Sphere`) "NoCollision")
      (return (`self.Item Type`)))))

(fn `UserConstructionScript`)